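; Test game mode for a clue game that judges the player's clue choices as a win or loss.
; On BeginPlay it shows a controls widget, gathers all BP_Clue actors and records each one's IsImportant flag.
; SetGameState counts submitted entries matching those flags by index, then CheckGameState compares the count to ClueScore and shows a three-second won or lost prompt.
; The name-sort event is empty and its loop is disconnected, so clues keep GetAllActorsOfClass order.
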(event Custom|Get%20All%20Clue%20Actors
  (bind _outactors (Actor|GetAllActorsOfClass "/Game/Dynamic/Blueprints/Actors/BP_Clue.BP_Clue_C"))
  (bind _output_get (Variables|Default|SetTemp%20Clue%20Actor%20List _outactors))
  (Variables|Default|SetSorted%20Clue%20Actor%20List _output_get))

(event Custom|Set%20Clue%20Bool%20List
  (for (_array_element _array_index) (Variables|Default|GetSorted%20Clue%20Actor%20List)
    (Utilities|Array|SetArrayElem (Variables|Default|GetClue%20Importance%20List) _array_index (Variables|/Game/Dynamic/Blueprints/Actors/BP_Clue.BP_Clue_C|GetisImportant _array_element))))

(event Custom|Sort%20Clue%20Actor%20List%20by%20Name)

(event Custom|Set%20Game%20State
  (params (Input%20Clue%20List :type Array%20of%20Booleans))
  (Variables|Default|SetPlayerClueScore 0)
  (for (_array_element _array_index) Input%20Clue%20List
    (Development|PrintString (Utilities|String|ToString(Boolean) _array_element))
    (if (== _array_element (Utilities|Array|Get(acopy) (Variables|Default|GetClue%20Importance%20List) _array_index))
      (Math|Integer|IncrementInt (Variables|Default|GetPlayerClueScore))))
  (CallFunction|CheckGameState)
  (Development|PrintString (Utilities|String|ToString(Integer) (Variables|Default|GetPlayerClueScore))))

(event Custom|Check%20Game%20State
  (bind _returnvalue (Game|GetPlayerController 0))
  (if (== (Variables|Default|GetPlayerClueScore) (Variables|Default|GetClueScore))
    (bind _returnvalue_2 (UserInterface|CreateWidget "/Game/Dynamic/UI/WB_GameWonPrompt.WB_GameWonPrompt_C" _returnvalue))
    (UserInterface|Viewport|AddtoViewport _returnvalue_2 0)
    (Utilities|FlowControl|Delay 3.0)
    (Widget|RemovefromParent _returnvalue_2)
    (else
      (bind _returnvalue_3 (UserInterface|CreateWidget "/Game/Dynamic/UI/WB_GameLostPrompt.WB_GameLostPrompt_C" _returnvalue))
      (UserInterface|Viewport|AddtoViewport _returnvalue_3 0)
      (Utilities|FlowControl|Delay 3.0)
      (Widget|RemovefromParent _returnvalue_3))))

(event EventBeginPlay
  (bind _returnvalue (UserInterface|CreateWidget "/Game/Dynamic/UI/WB_ControlsBox.WB_ControlsBox_C" (Game|GetPlayerController 0)))
  (UserInterface|Viewport|AddtoViewport _returnvalue 0)
  (CallFunction|GetAllClueActors)
  (CallFunction|SortClueActorListbyName)
  (CallFunction|SetClueBoolList))

(fn ConstructionScript)