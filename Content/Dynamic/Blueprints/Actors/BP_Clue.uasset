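; BP_Clue is an interactable clue actor that tells the player whether it is important.
; Interact marks it interacted and shows a correct or incorrect prompt based on IsImportant.
; A DoOnce blocks repeats until the timed prompt is removed, then the Interacted dispatcher fires.
; InteractCollision overlaps toggle the hint widget through a FlipFlop without filtering actors, while CanInteract always returns false.
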(event OnComponentBeginOverlap(InteractCollision)
  (params (OverlappedComponent :type Primitive%20Component%20Object%20Reference) (OtherActor :type Actor%20Object%20Reference) (OtherComp :type Primitive%20Component%20Object%20Reference) (OtherBodyIndex :type Integer) (bFromSweep :type Boolean) (SweepResult :type Hit%20Result%20Structure%20%28by%20ref%29))
  (CallFunction|ToggleInteractWidget))

(event OnComponentEndOverlap(InteractCollision)
  (params (OverlappedComponent :type Primitive%20Component%20Object%20Reference) (OtherActor :type Actor%20Object%20Reference) (OtherComp :type Primitive%20Component%20Object%20Reference) (OtherBodyIndex :type Integer))
  (CallFunction|ToggleInteractWidget))

(event Custom|Reset%20Interact
  (Utilities|FlowControl|DoOnce false) ; enters at Reset
)

(event Custom|Toggle%20Interact%20Widget
  (bind _isa (Utilities|FlowControl|FlipFlop)
    (:A
      _)
    (:B
      _))
  (Development|SetHiddeninGame (Variables|Default|GetWidget) (not _isa) false))

(event EventBeginPlay)

(event EventInteract
  (Utilities|FlowControl|DoOnce false
    (:Completed
      (Variables|Default|SetisInteracted true)
      (if (Variables|Default|GetisImportant)
        (Variables|Default|SetWidget%20Prompt (Variables|Default|GetWidget%20Correct%20Prompt))
        (else
          (Variables|Default|SetWidget%20Prompt (Variables|Default|GetWidget%20Incorrect%20Prompt))))
      (bind _returnvalue (UserInterface|CreateWidget (Variables|Default|GetWidget%20Prompt) (Game|GetPlayerController 0)))
      (UserInterface|Viewport|AddtoViewport _returnvalue 0)
      (Utilities|FlowControl|Delay 3.0)
      (Widget|RemovefromParent _returnvalue)
      (CallFunction|ResetInteract)
      (Default|CallInteracted))))

(fn ConstructionScript)

(fn CanInteract
  (return false))